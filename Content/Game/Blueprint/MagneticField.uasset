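; MagneticField is a trigger actor that destroys positive charges, negative charges and non-Anti celestive charges entering its Box.
; The overlap event casts to each charge class in turn, destroys the match and routes into a shared DoOnce.
; The first destruction starts a one-time sequence of delayed 2D sounds and a temporary W_Text widget prompting the player to press F to open documentation.
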(event OnComponentBeginOverlap(Box)
  (params (OverlappedComponent :type Primitive%20Component%20Object%20Reference) (OtherActor :type Actor%20Object%20Reference) (OtherComp :type Primitive%20Component%20Object%20Reference) (OtherBodyIndex :type Integer) (bFromSweep :type Boolean) (SweepResult :type Hit%20Result%20Structure%20%28by%20ref%29))
  (bind _asa_positive_charge_bp (Utilities|Casting|CastToA_PositiveChargeBP OtherActor)
    (:then
      (Actor|DestroyActor _asa_positive_charge_bp)
      (Utilities|FlowControl|DoOnce false :!label _label
        (:Completed
          (Audio|PlaySound2D "/Game/Game/ImportedSound/M_3.M_3" 1e+01 1.0 0.0 0 0)
          (Utilities|FlowControl|Delay 8.0)
          (bind _returnvalue (UserInterface|CreateWidget "/Game/Game/Widget/W_Text.W_Text_C"))
          (Variables|/Script/UMG.TextBlock|SetText (Variables|/Game/Game/Widget/W_Text.W_Text_C|GetTextBlock_0 _returnvalue) "Press F to Open Documentation ")
          (UserInterface|Viewport|AddtoViewport _returnvalue 0)
          (Audio|PlaySound2D "/Game/Game/ImportedSound/M2_Next.M2_Next" 1e+01 1.0 1e+01 0 0)
          (Utilities|FlowControl|Delay 7.0)
          (Widget|RemovefromParent _returnvalue))))
    (:CastFailed
      (bind _asa_negative_charge_bp (Utilities|Casting|CastToA_NegativeChargeBP OtherActor)
        (:then
          (Actor|DestroyActor _asa_negative_charge_bp)
          (goto _label))
        (:CastFailed
          (bind _asa_celestive_charge_bp (Utilities|Casting|CastToA_CelestiveChargeBP OtherActor))
          (if (not (Variables|/Script/GameJam.A_ChargeBase|Getanti _asa_celestive_charge_bp))
            (Actor|DestroyActor _asa_celestive_charge_bp)
            (goto _label)))))))

(event EventBeginPlay)

(event Collision|EventActorBeginOverlap
  (params (OtherActor :type Actor%20Object%20Reference)))

(event EventTick
  (params (DeltaSeconds :type Float%20%28single-precision%29)))

(fn ConstructionScript)